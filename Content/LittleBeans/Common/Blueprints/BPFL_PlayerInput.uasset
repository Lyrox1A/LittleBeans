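; Blueprint function library that switches the first local player between game and UI input modes.
; Game mode sets game-only input, while UI mode sets game-and-UI input with focus on a given widget.
; It asks the game mode whether a gamepad is in use and only toggles mouse cursor visibility when it is not.
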(fn `SwitchInputMode`
  (params (NewInputMode :type "/Game/LittleBeans/Common/Blueprints/Enum_InputMode Enum" :default "NewEnumerator0") (InWidgetToFocus :type "Widget Object Reference"))
  (switch `/Game/LittleBeans/Common/Blueprints/Enum_InputMode` NewInputMode
    (:`NewEnumerator0`
      (`WidgetBlueprintLibrary.SetInputMode_GameOnly` (`GameplayStatics.GetPlayerController` null))
      (bind _bisusinggamepad (message `/Game/LittleBeans/Core/BPI_GameMode.GetIsUsingGamepad` (`GameplayStatics.GetGameMode` null)))
      (if _bisusinggamepad
        (return)
        (else
          (set `PlayerController.bShowMouseCursor` false (`GameplayStatics.GetPlayerController` null))
          (return))))
    (:`NewEnumerator1`
      (`WidgetBlueprintLibrary.SetInputMode_GameAndUIEx` (`GameplayStatics.GetPlayerController` null) InWidgetToFocus)
      (bind _bisusinggamepad_2 (message `/Game/LittleBeans/Core/BPI_GameMode.GetIsUsingGamepad` (`GameplayStatics.GetGameMode` null)))
      (if _bisusinggamepad_2
        (return)
        (else
          (set `PlayerController.bShowMouseCursor` true (`GameplayStatics.GetPlayerController` null))
          (return))))))