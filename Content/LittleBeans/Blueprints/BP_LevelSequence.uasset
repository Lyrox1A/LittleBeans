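; BP_LevelSequence plays the Cutscene00 level sequence as an intro cutscene when play begins.
; BeginPlay passes through a DoOnce, disables input on player character 0 and starts the sequence player.
; A hard-coded delay, rather than a sequence-finished event, then stops playback and restores input.
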(event `self.ReceiveBeginPlay`
  (bind _sequenceplayer (`LevelSequenceActor.SequencePlayer` (`self.Cutscene_00`)))
  (`/Engine/EditorBlueprintResources/StandardMacros.DoOnce` false
    (:`Completed`
      (`self.DisableInput` (`GameplayStatics.GetPlayerCharacter` 0) (`GameplayStatics.GetPlayerController` 0))
      (`MovieSceneSequencePlayer.Play` _sequenceplayer)
      (`KismetSystemLibrary.Delay` 7.5)
      (`MovieSceneSequencePlayer.Stop` _sequenceplayer)
      (`self.EnableInput` (`GameplayStatics.GetPlayerCharacter` 0) (`GameplayStatics.GetPlayerController` 0)))))

(fn `UserConstructionScript`)