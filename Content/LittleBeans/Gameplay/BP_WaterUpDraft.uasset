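; Water updraft actor that launches the third-person character upward while it is inside the collision volume, with looping FMOD audio started at BeginPlay.
; Overlap sets a flag and starts a looping timer that, while flagged, adds UpDraftRange to vertical velocity and plays a 2D sound.
; A DoOnce with a delayed reset spaces out boosts.
; Leaving clears the flag but never the timer.
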(event `self.ReceiveBeginPlay`
  (`FMODAudioComponent.Play` (`self.FMODAudio`)))

(event `self.Collision.OnComponentBeginOverlap`
  (params (OverlappedComponent :type "PrimitiveComponent Object Reference") (OtherActor :type "Actor Object Reference") (OtherComp :type "PrimitiveComponent Object Reference") (OtherBodyIndex :type Integer) (bFromSweep :type Boolean) (SweepResult :type "HitResult Structure (by ref)"))
  (bind _asbp_third_person_character (cast `/Game/ThirdPerson/Blueprints/BP_ThirdPersonCharacter` OtherActor))
  (set `self.bWaterUpDraft` true)
  (`KismetSystemLibrary.K2_SetTimerDelegate` (delegate `Activate Water Fountain`) 0.1 true))

(event `Activate Water Fountain`
  (if (`self.bWaterUpDraft`)
    (`/Engine/EditorBlueprintResources/StandardMacros.DoOnce` false :!label _label
      (:`Completed`
        (`FMODBlueprintStatics.PlayEvent2D` "/Game/FMOD/Events/WaterUpdraft.WaterUpdraft")
        (bind _charactermovement (`Character.CharacterMovement` (stale `self.Collision.OnComponentBeginOverlap` _asbp_third_person_character)))
        (bind (_velocity_x _velocity_y _velocity_z) (`KismetMathLibrary.BreakVector` (`MovementComponent.Velocity` _charactermovement)))
        (set `MovementComponent.Velocity` (`KismetMathLibrary.MakeVector` _velocity_x _velocity_y (+ _velocity_z (`self.UpDraftRange`))) _charactermovement)
        (`KismetSystemLibrary.Delay` 2.0)
        (goto _label :!via `Reset`)))))

(event `self.Collision.OnComponentEndOverlap`
  (params (OverlappedComponent :type "PrimitiveComponent Object Reference") (OtherActor :type "Actor Object Reference") (OtherComp :type "PrimitiveComponent Object Reference") (OtherBodyIndex :type Integer))
  (cast `/Game/ThirdPerson/Blueprints/BP_ThirdPersonCharacter` OtherActor)
  (set `self.bWaterUpDraft` false))

(fn `UserConstructionScript`)