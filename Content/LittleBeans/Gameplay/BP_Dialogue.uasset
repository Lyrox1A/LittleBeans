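; BP_Dialogue is a trigger actor that plays a multi-line conversation and rewards its completion with a collectable.
; Overlapping its collision registers it as the player's activatable object and shows a control hint; leaving hides the hint and ends the dialogue.
; Each TriggerReceiver call sends the next speaker/text pair to the game mode through messages.
; After the last line, it spawns BP_Collectable in its place and destroys itself.
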(event `self.Collsion.OnComponentBeginOverlap`
  (params (OverlappedComponent :type "PrimitiveComponent Object Reference") (OtherActor :type "Actor Object Reference") (OtherComp :type "PrimitiveComponent Object Reference") (OtherBodyIndex :type Integer) (bFromSweep :type Boolean) (SweepResult :type "HitResult Structure (by ref)"))
  (if (== (`GameplayStatics.GetObjectClass` OtherActor) "/Game/ThirdPerson/Blueprints/BP_ThirdPersonCharacter.BP_ThirdPersonCharacter_C")
    (message `/Game/LittleBeans/Blueprints/BPI_PlayerCharacter.is in Activatable Range` (`GameplayStatics.GetPlayerCharacter` 0) self true)
    (message `/Game/LittleBeans/UI/ControlHints/BPI_ControlHints.ShowControlHint` (`GameplayStatics.GetGameMode`) "" false true)))

(event `self.Collsion.OnComponentEndOverlap`
  (params (OverlappedComponent :type "PrimitiveComponent Object Reference") (OtherActor :type "Actor Object Reference") (OtherComp :type "PrimitiveComponent Object Reference") (OtherBodyIndex :type Integer))
  (if (== (`GameplayStatics.GetObjectClass` OtherActor) "/Game/ThirdPerson/Blueprints/BP_ThirdPersonCharacter.BP_ThirdPersonCharacter_C")
    (message `/Game/LittleBeans/UI/ControlHints/BPI_ControlHints.ShowControlHint` (`GameplayStatics.GetGameMode`) "" false false)
    (message `/Game/LittleBeans/Core/BPI_GameMode.EndDialogue` (`GameplayStatics.GetGameMode`))))

(event `/Game/LittleBeans/Gameplay/BPI_TriggerReceiver.TriggerReceiver`
  (params (TriggerRef :type "Actor Object Reference") (bShouldRetrigger :type Boolean) (Delay :type "Float (double-precision)"))
  (if (not (>= (`self.DialogueIndex`) (`KismetArrayLibrary.Array_Length` (`self.DialogueText`))))
    (message `/Game/LittleBeans/Core/BPI_GameMode.TriggerDialgue` (`GameplayStatics.GetGameMode`) (`|GetArrayItem` (`self.DialogueSpeaker`) (`self.DialogueIndex`)) (`|GetArrayItem` (`self.DialogueText`) (`self.DialogueIndex`)))
    (`/Engine/EditorBlueprintResources/StandardMacros.IncrementInt` (`self.DialogueIndex`))
    (else
      (message `/Game/LittleBeans/Core/BPI_GameMode.EndDialogue` (`GameplayStatics.GetGameMode`))
      (set `self.DialogueIndex` 0)
      (`|SpawnActorFromClass` "/Game/LittleBeans/Gameplay/Pickups/BP_Collectable.BP_Collectable_C" (`self.GetTransform`) "Undefined" "OverrideRootScale" null null)
      (`self.K2_DestroyActor`))))

(fn `UserConstructionScript`)