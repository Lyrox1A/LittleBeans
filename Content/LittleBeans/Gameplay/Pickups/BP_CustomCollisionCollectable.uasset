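; A collectable pickup that spins in place and removes itself when collected through its Collision component.
; On BeginPlay it gives RotatingMovement a random pitch and yaw rate, so instances tumble differently.
; When an actor of one specific class begins overlapping, it sends CollectedMessage with a fixed enum value to the game mode and player character 0, then destroys itself.
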(event `self.ReceiveBeginPlay`
  ;[1 1 1] Begin Play
  (set `RotatingMovementComponent.RotationRate` (`KismetMathLibrary.MakeRotator` 0.0 (`KismetMathLibrary.RandomFloatInRange` 100.0 180.0) (`KismetMathLibrary.RandomFloatInRange` 100.0 180.0)) (`self.RotatingMovement`)))

(event `self.Collision.OnComponentBeginOverlap`
  (params (OverlappedComponent :type "PrimitiveComponent Object Reference") (OtherActor :type "Actor Object Reference") (OtherComp :type "PrimitiveComponent Object Reference") (OtherBodyIndex :type Integer) (bFromSweep :type Boolean) (SweepResult :type "HitResult Structure (by ref)"))
  ;[1 1 1] Begin Overlap
  (if (== (`GameplayStatics.GetObjectClass` OtherActor) null)
    (message `/Game/LittleBeans/Gameplay/Pickups/BPI_Pickup.Collected` (`GameplayStatics.GetGameMode`) "NewEnumerator1")
    (message `/Game/LittleBeans/Gameplay/Pickups/BPI_Pickup.Collected` (`GameplayStatics.GetPlayerCharacter` 0) "NewEnumerator1")
    (`self.K2_DestroyActor`)))

(fn `UserConstructionScript`)