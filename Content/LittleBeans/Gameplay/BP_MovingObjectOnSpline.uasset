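; Actor that moves an object along a spline with FMOD audio, starting on a trigger event or at BeginPlay.
; A looping 0.01-second timer advances or rewinds the distance by speed times world delta and repositions the object.
; At the ends it wraps on closed splines or ping-pongs when looping, otherwise stops.
; Interruptable objects reverse on triggers; others ignore them until finished, re-arming only if retriggerable.
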(event `self.ReceiveBeginPlay`
  ;[0.3462 1 0.3532] Begin Play
  (`FMODAudioComponent.Play` (`self.FMODAudio`))
  (`SceneComponent.K2_SetWorldLocation` (`self.MovingObject`) (`SplineComponent.GetLocationAtDistanceAlongSpline` (`self.Spline`) 0.0 "World") false false)
  (set `self.CurrentDistance` 0.0)
  (if (`self.StartAwake`)
    (`self.Start Awake`)))

(event `/Game/LittleBeans/Gameplay/BPI_TriggerReceiver.TriggerReceiver`
  (params (TriggerRef :type "Actor Object Reference") (bShouldRetrigger :type Boolean) (Delay :type "Float (double-precision)"))
  ;[0.1667 0.1667 0.1667] Receive Trigger Event
  (if (`self.bInteruptable`) :!label _label
    (`KismetSystemLibrary.K2_ClearAndInvalidateTimerHandle` (`self.MoveObjectTimer`))
    (`self.ResetObjectMovement`)
    (`/Engine/EditorBlueprintResources/StandardMacros.FlipFlop`
      (:`A`
        (set `self.bMovingForwad` true))
      (:`B`
        (set `self.bMovingForwad` false)))
    (else
      (`/Engine/EditorBlueprintResources/StandardMacros.DoOnce` false :!label _label_2
        (:`Completed`
          (set `self.Should Retrigger` bShouldRetrigger)))))
  (bind _returnvalue (`KismetSystemLibrary.K2_SetTimerDelegate` (delegate `IncreaseDistance`) 0.01 true))
  (set `self.MoveObjectTimer` _returnvalue))

(event `ResetObjectMovement`
  ;[0.1667 0.1667 0.1667] Receive Trigger Event
  (goto _label_2 :!via `Reset`))

(event `Start Awake`
  ;[0.1667 0.1667 0.1667] Receive Trigger Event
  (goto _label))

(event `IncreaseDistance`
  ;[0.1667 0.1667 0.1667] Receive Trigger Event
  (if (or (and (< (`self.CurrentDistance`) (`SplineComponent.GetSplineLength` (`self.Spline`))) (`self.bMovingForwad`)) (and (>= (`self.CurrentDistance`) 0.0) (not (`self.bMovingForwad`))))
    (bind _newdistance (`self.CalculateDistance` (`self.bMovingForwad`)))
    (bind _output_get (set `self.CurrentDistance` _newdistance))
    (`SceneComponent.K2_SetWorldLocation` (`self.MovingObject`) (`SplineComponent.GetLocationAtDistanceAlongSpline` (`self.Spline`) _output_get "World") false false)
    (elif (and (`SplineComponent.IsClosedLoop` (`self.Spline`)) (`self.bLoopOnSpline`))
      (set `self.CurrentDistance` 0.0)
      (elif (`self.bLoopOnSpline`)
        (`/Engine/EditorBlueprintResources/StandardMacros.FlipFlop`
          (:`A`
            (set `self.bMovingForwad` false))
          (:`B`
            (set `self.bMovingForwad` true)))
        (else
          (`KismetSystemLibrary.K2_ClearAndInvalidateTimerHandle` (`self.MoveObjectTimer`))
          (if (`self.Should Retrigger`)
            (`self.ResetObjectMovement`)
            (`/Engine/EditorBlueprintResources/StandardMacros.FlipFlop`
              (:`A`
                (set `self.bMovingForwad` false))
              (:`B`
                (set `self.bMovingForwad` true)))))))))

(fn `CalculateDistance`
  (params (bMovingForwad :type Boolean))
  (returns (NewDistance :type "Float (double-precision)"))
  (if bMovingForwad
    (return (+ (`self.CurrentDistance`) (* (`self.Speed`) (`GameplayStatics.GetWorldDeltaSeconds`))))
    (else
      (return (- (`self.CurrentDistance`) (* (`self.Speed`) (`GameplayStatics.GetWorldDeltaSeconds`)))))))

(fn `UserConstructionScript`)