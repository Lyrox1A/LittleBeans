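; Boost platform actor that bounces the player character straight up on contact.
; On BeginPlay it caches player 0 as a BP_ThirdPersonCharacter.
; When an actor of exactly that class overlaps the Collision component, it plays the BouncyTrashCan 2D sound event and launches the cached player, not the overlapping actor.
; The launch overrides vertical velocity with LaunchRange and keeps horizontal momentum.
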(event `self.ReceiveBeginPlay`
  (bind _asbp_third_person_character (cast `/Game/ThirdPerson/Blueprints/BP_ThirdPersonCharacter` (`GameplayStatics.GetPlayerCharacter` 0)))
  (set `self.Player Character ` _asbp_third_person_character))

(event `self.Collision.OnComponentBeginOverlap`
  (params (OverlappedComponent :type "PrimitiveComponent Object Reference") (OtherActor :type "Actor Object Reference") (OtherComp :type "PrimitiveComponent Object Reference") (OtherBodyIndex :type Integer) (bFromSweep :type Boolean) (SweepResult :type "HitResult Structure (by ref)"))
  (if (== (`GameplayStatics.GetObjectClass` OtherActor) "/Game/ThirdPerson/Blueprints/BP_ThirdPersonCharacter.BP_ThirdPersonCharacter_C")
    (`FMODBlueprintStatics.PlayEvent2D` "/Game/FMOD/Events/BouncyTrashCan.BouncyTrashCan")
    (`Character.LaunchCharacter` (`self.Player Character `) (`KismetMathLibrary.MakeVector` 0.0 0.0 (`self.LaunchRange`)) false true)))

(fn `UserConstructionScript`)