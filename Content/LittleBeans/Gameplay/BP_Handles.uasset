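; BP_Handles is an obstacle or prop that swings a mesh back and forth in yaw between configurable left and right limits.
; A looping 0.01-second timer, rather than Tick, steps the mesh's relative rotation by a Speed-scaled amount in the current direction.
; At each limit it plays FMOD audio, pauses that timer for PauseTime via a one-shot timer, then reverses direction.
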(event `self.ReceiveBeginPlay`
  (set `self.CurrentRotation` (`SceneComponent.RelativeRotation` (`self.SM_SwingObject`)))
  (set `self.MinRotation` (`KismetMathLibrary.MakeRotator` 90.0 0.0 (* (`self.MaxLeft`) -1.0)))
  (set `self.MaxRotation` (`KismetMathLibrary.MakeRotator` 90.0 0.0 (`self.MaxRight`)))
  (`self.StartTimer`))

(event `StartTimer`
  (bind _returnvalue (`KismetSystemLibrary.K2_SetTimerDelegate` (delegate `IncreaseRotation`) 0.01 true))
  (set `self.TimerHandleRef` _returnvalue))

(event `IncreaseRotation`
  (if (`self.bRotatingForward`)
    (`self.RotateForward`)
    (else
      (`self.RotateBackward`))))

(event `PauseHandle`
  (`KismetSystemLibrary.PrintText` "SOUND")
  (`FMODAudioComponent.Play` (`self.FMODAudio`))
  (`KismetSystemLibrary.K2_PauseTimerHandle` (`self.TimerHandleRef`))
  (`KismetSystemLibrary.K2_SetTimerDelegate` (delegate `UnpauseHandle`) (`self.PauseTime`)))

(event `UnpauseHandle`
  (`KismetSystemLibrary.K2_UnPauseTimerHandle` (`self.TimerHandleRef`)))

(fn `RotateBackward`
  (bind (_currentrotation_roll _currentrotation_pitch _currentrotation_yaw) (`KismetMathLibrary.BreakRotator` (`self.CurrentRotation`)))
  (bind (_currentrotation_roll_2 _currentrotation_pitch_2 _currentrotation_yaw_2) (`KismetMathLibrary.BreakRotator` (`self.CurrentRotation`)))
  (bind (_minrotation_roll _minrotation_pitch _minrotation_yaw) (`KismetMathLibrary.BreakRotator` (`self.MinRotation`)))
  (if (> _currentrotation_yaw _minrotation_yaw)
    (bind _output_get (set `self.CurrentRotation` (`KismetMathLibrary.MakeRotator` _currentrotation_roll_2 _currentrotation_pitch_2 (- _currentrotation_yaw_2 (/ (`self.Speed`) 100.0)))))
    (`SceneComponent.K2_SetRelativeRotation` (`self.SM_SwingObject`) _output_get false false)
    (else
      (`self.PauseHandle`)
      (set `self.bRotatingForward` true))))

(fn `RotateForward`
  (bind (_maxrotation_roll _maxrotation_pitch _maxrotation_yaw) (`KismetMathLibrary.BreakRotator` (`self.MaxRotation`)))
  (bind (_currentrotation_roll _currentrotation_pitch _currentrotation_yaw) (`KismetMathLibrary.BreakRotator` (`self.CurrentRotation`)))
  (bind (_currentrotation_roll_2 _currentrotation_pitch_2 _currentrotation_yaw_2) (`KismetMathLibrary.BreakRotator` (`self.CurrentRotation`)))
  (if (< _currentrotation_yaw _maxrotation_yaw)
    (bind _output_get (set `self.CurrentRotation` (`KismetMathLibrary.MakeRotator` _currentrotation_roll_2 _currentrotation_pitch_2 (+ _currentrotation_yaw_2 (/ (`self.Speed`) 100.0)))))
    (`SceneComponent.K2_SetRelativeRotation` (`self.SM_SwingObject`) _output_get false false)
    (else
      (`self.PauseHandle`)
      (set `self.bRotatingForward` false))))

(fn `UserConstructionScript`)