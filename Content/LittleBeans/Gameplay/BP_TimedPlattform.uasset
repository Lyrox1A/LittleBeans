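; BP_TimedPlattform is a platform that falls away a set time after the player character steps on it.
; The first overlap shows a countdown widget and starts a timer that plays a timeline, lowering the cube and fading its dynamic material before disabling collision.
; It returns by reversing the timeline, either after a respawn delay or via TriggerReceiver, depending on ResetWithTrigger.
; DoOnce gates block repeat triggers until each transition finishes.
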(event `self.ReceiveBeginPlay`
  ;[0.3632 1 0.3245] Begin Play
  (bind _returnvalue (`MaterialInstanceDynamic.K2_GetVectorParameterValue` (`self.PlattformMaterial`) "Color"))
  (set `self.BaseColor` _returnvalue)
  (set `self.PlattformStartLocation` (`SceneComponent.K2_GetComponentLocation` (`self.Cube`)))
  (`TimelineComponent.SetPlayRate` (`self.PlattformFade`) (`self.FallFadeSpeed`)))

(event `self.Collision.OnComponentBeginOverlap`
  (params (OverlappedComponent :type "PrimitiveComponent Object Reference") (OtherActor :type "Actor Object Reference") (OtherComp :type "PrimitiveComponent Object Reference") (OtherBodyIndex :type Integer) (bFromSweep :type Boolean) (SweepResult :type "HitResult Structure (by ref)"))
  ;[1 1 1] Begin Overlap
  (if (== (`GameplayStatics.GetObjectClass` OtherActor) "/Game/ThirdPerson/Blueprints/BP_ThirdPersonCharacter.BP_ThirdPersonCharacter_C")
    (`/Engine/EditorBlueprintResources/StandardMacros.DoOnce` false :!label _label
      (:`Completed`
        (bind _returnvalue (`|CreateWidget` "/Game/LittleBeans/UI/WBP_Countdown.WBP_Countdown_C" null (`self.TimeTillFall`)))
        (`UserWidget.AddToViewport` _returnvalue 0)
        (`KismetSystemLibrary.K2_SetTimerDelegate` (delegate `PlattformFall`) (`self.TimeTillFall`))))))

(event `PlattformReset`
  ;[1 1 1] Begin Overlap
  (goto _label :!via `Reset`))

(event `PlattformFall`
  ;[1 1 1] Begin Overlap
  (`self.TogglePlattform` true)
  (if (not (`self.bResetWithTrigger`))
    (`KismetSystemLibrary.K2_SetTimerDelegate` (delegate `RespawnPlattform`) (`self.RespawnTime`))))

(event `RespawnPlattform`
  ;[1 1 1] Begin Overlap
  (`self.TogglePlattform` false))

(event `TogglePlattform`
  (params (bHide :type Boolean))
  (bind (_basecolor_r _basecolor_g _basecolor_b) (break `LinearColor` (`self.BaseColor`)))
  ;[1 1 1] Begin Overlap
  (if bHide
    (bind (_direction _alpha_0_1) (`Timeline|PlattformFade` :!via `PlayFromStart` :!label _label_2)
      (:`Update`
        ;;[1 1 1] Plattform Movement
        (`SceneComponent.K2_SetWorldLocation` (`self.Cube`) (`KismetMathLibrary.VLerp` (`self.PlattformStartLocation`) (- (`self.PlattformStartLocation`) (`KismetMathLibrary.MakeVector` 0.0 0.0 (`self.FallAmount`))) _alpha_0_1) false false)
        ;;[1 1 1] ColorFade
        (`MaterialInstanceDynamic.SetVectorParameterValue` (`self.PlattformMaterial`) "Color" (make `LinearColor` _basecolor_r _basecolor_g _basecolor_b (- 1.0 _alpha_0_1))))
      (:`Finished`
        (switch `ETimelineDirection` _direction
          (:`Forward`
            (`PrimitiveComponent.SetCollisionEnabled` (`self.Cube`) "NoCollision")
            (`self.ResetTriggerFadeIn`))
          (:`Backward`
            (`PrimitiveComponent.SetCollisionEnabled` (`self.Cube`) "QueryAndPhysics")
            (`self.PlattformReset`)))))
    (else
      (goto _label_2 :!via `ReverseFromEnd`))))

(event `/Game/LittleBeans/Gameplay/BPI_TriggerReceiver.TriggerReceiver`
  (params (TriggerRef :type "Actor Object Reference") (bShouldRetrigger :type Boolean) (Delay :type "Float (double-precision)"))
  ;[1 1 1] Begin Overlap
  ;;[1 1 1] Trigger Event
  (if (`self.bResetWithTrigger`)
    (`/Engine/EditorBlueprintResources/StandardMacros.DoOnce` true :!label _label_3
      (:`Completed`
        (`self.TogglePlattform` false)))))

(event `ResetTriggerFadeIn`
  ;[1 1 1] Begin Overlap
  ;;[1 1 1] Trigger Event
  (goto _label_3 :!via `Reset`))

(fn `UserConstructionScript`
  (bind _returnvalue (`PrimitiveComponent.CreateDynamicMaterialInstance` (`self.Cube`) 0 "/Game/LittleBeans/Material/MI_Transparent_FallingPlattform.MI_Transparent_FallingPlattform" "None"))
  (set `self.PlattformMaterial` _returnvalue))