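; BP_Checkpoint is a placeable checkpoint that registers its location with the game mode when the player character touches it.
; Its Collision overlap checks for the exact BP_ThirdPersonCharacter class, then passes the root's world transform to the game mode through SetCheckpointMessage.
; Any other overlapping actor only triggers a debug "Hi" print.
; GetCurrentPickups and GetIsUsingGamepad are stubs returning default values.
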(event `self.Collision.OnComponentBeginOverlap`
  (params (OverlappedComponent :type "PrimitiveComponent Object Reference") (OtherActor :type "Actor Object Reference") (OtherComp :type "PrimitiveComponent Object Reference") (OtherBodyIndex :type Integer) (bFromSweep :type Boolean) (SweepResult :type "HitResult Structure (by ref)"))
  ;[1 1 1] Begin Overlap
  (if (== (`GameplayStatics.GetObjectClass` OtherActor) "/Game/ThirdPerson/Blueprints/BP_ThirdPersonCharacter.BP_ThirdPersonCharacter_C")
    (message `/Game/LittleBeans/Core/BPI_GameMode.SetCheckpoint` (`GameplayStatics.GetGameMode`) (`SceneComponent.K2_GetComponentToWorld` (`self.DefaultSceneRoot`)))
    (else
      (`KismetSystemLibrary.PrintText` "Hi"))))

(fn `GetCurrentPickups`
  (returns (CurrentPickups :type Integer))
  (return 0))

(fn `GetIsUsingGamepad`
  (returns (bIsUsingGamepad :type Boolean))
  (return false))

(fn `UserConstructionScript`)