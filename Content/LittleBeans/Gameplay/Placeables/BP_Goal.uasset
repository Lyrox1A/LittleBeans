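; BP_Goal is a placeable goal that wins the game when the third-person player character overlaps its collision.
; On BeginPlay it shows a "Goal!" player hint through its widget component.
; The overlap clears the hint, fades out the music bus, plays the game-won music and calls GameWonMessage on the game mode.
; GetCurrentPickups and GetIsUsingGamepad are stubs returning default values.
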(event `self.ReceiveBeginPlay`
  ;[0.4064 1 0.3939] Begin Play
  (bind _returnvalue (`|CreateWidget` "/Game/LittleBeans/UI/WBP_PlayerHint.WBP_PlayerHint_C" null "Goal!"))
  (set `self.GoalHintRef` _returnvalue)
  (`WidgetComponent.SetWidget` (`self.Widget`) (`self.GoalHintRef`)))

(event `self.Collision.OnComponentBeginOverlap`
  (params (OverlappedComponent :type "PrimitiveComponent Object Reference") (OtherActor :type "Actor Object Reference") (OtherComp :type "PrimitiveComponent Object Reference") (OtherBodyIndex :type Integer) (bFromSweep :type Boolean) (SweepResult :type "HitResult Structure (by ref)"))
  ;[1 1 1] Begin Overlap
  (if (== (`GameplayStatics.GetObjectClass` OtherActor) "/Game/ThirdPerson/Blueprints/BP_ThirdPersonCharacter.BP_ThirdPersonCharacter_C")
    (`FMODBlueprintStatics.BusStopAllEvents` "/Game/FMOD/Buses/Music.Music" "ALLOWFADEOUT")
    (`FMODBlueprintStatics.PlayEvent2D` "/Game/FMOD/Events/GameWonMusic.GameWonMusic")
    (`WidgetComponent.SetWidget` (`self.Widget`) null)
    (message `/Game/LittleBeans/Core/BPI_GameMode.GameWon` (`GameplayStatics.GetGameMode`))))

(fn `GetCurrentPickups`
  (returns (CurrentPickups :type Integer))
  (return 0))

(fn `GetIsUsingGamepad`
  (returns (bIsUsingGamepad :type Boolean))
  (return false))

(fn `UserConstructionScript`)