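; Game mode for LittleBeans that acts as the central hub for game state and UI.
; Creates and toggles overlay, pause, win, settings, cheat and dialogue widgets, managing pause state, input mode and the player's dialogue flag.
; Stores the checkpoint, seeded from the player start, for respawns, and counts pickups for the overlay.
; Tracks gamepad use, forwards control hints to the overlay and applies Master, Music and SFX volumes through audio VCAs.
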(event `self.ReceiveBeginPlay`
  (bind _returnvalue (`GameplayStatics.GetPlayerController` 0))
  ;[0.1961 1 0.2124] Begin Play
  (`self.EnableInput` _returnvalue)
  (`WidgetBlueprintLibrary.SetInputMode_GameOnly` _returnvalue)
  (set `self.CurrentCheckpoint` (`self.GetTransform` (`self.K2_FindPlayerStart` null)))
  (bind _returnvalue_2 (`|CreateWidget` "/Game/LittleBeans/UI/WBP_IngameOverlay.WBP_IngameOverlay_C"))
  (bind _output_get (set `self.IngameUIRef` _returnvalue_2))
  (`UserWidget.AddToViewport` _output_get 0))

(event `/Game/LittleBeans/Core/BPI_GameMode.TriggerPause`
  ;[1 1 1] Pause Game
  (if (not (`self.bIsGamePaused`)) :!label _label
    (`/Engine/EditorBlueprintResources/StandardMacros.IsValid` (`self.PauseMenuRef`)
      (:`Is Valid`
        _)
      (:`Is Not Valid`
        (bind _returnvalue (`|CreateWidget` "/Game/LittleBeans/UI/WBP_MenuContainer.WBP_MenuContainer_C" null "NewEnumerator0" false))
        (set `self.PauseMenuRef` _returnvalue)))
    (`UserWidget.AddToViewport` (`self.PauseMenuRef`) 0)
    (`/Game/LittleBeans/Common/Blueprints/BPFL_PlayerInput.SwitchInputMode` "NewEnumerator1" (`self.PauseMenuRef`))
    (`GameplayStatics.SetGamePaused` true)
    (set `self.bIsGamePaused` true)
    (else
      (`Widget.RemoveFromParent` (`self.PauseMenuRef`))
      (`/Game/LittleBeans/Common/Blueprints/BPFL_PlayerInput.SwitchInputMode` "NewEnumerator0" (`self.PauseMenuRef`))
      (`GameplayStatics.SetGamePaused` false)
      (set `self.bIsGamePaused` false))))

(event `/Game/LittleBeans/Core/BPI_GameMode.StartGame`
  ;[1 1 1] Start Game
  (message `/Game/LittleBeans/Core/BPI_GameInstance.ChangeLevel` (`GameplayStatics.GetGameInstance`) "NewEnumerator1"))

(event `InputAction|PauseMenu`
  (params (Key :type "Key Structure"))
  ;[1 1 1] Pause Game
  (:`Pressed`
    (goto _label)))

(event `/Game/LittleBeans/Core/BPI_GameMode.ExitGame`
  ;[1 1 1] Quit Game
  (`KismetSystemLibrary.QuitGame` null "Quit"))

(event `Event Show Control Hint`
  (params (ActionToHint :type String) (bGamepad :type Boolean) (bShow :type Boolean))
  ;[1 1 1] Control Hints
  (message `/Game/LittleBeans/UI/ControlHints/BPI_ControlHints.ShowControlHint` (`self.IngameUIRef`) ActionToHint (`self.Is Using Gamepad`) bShow))

(event `Event Switch Control Hint`
  (params (bGamepad :type Boolean))
  ;[1 1 1] Control Hints
  (message `/Game/LittleBeans/UI/ControlHints/BPI_ControlHints.SwitchControlHint` (`self.IngameUIRef`) bGamepad))

(event `/Game/LittleBeans/Core/BPI_GameMode.GameWon`
  ;[1 1 1] Game Won
  (bind _returnvalue (`|CreateWidget` "/Game/LittleBeans/UI/WBP_MenuContainer.WBP_MenuContainer_C" null "NewEnumerator2" false))
  (bind _output_get (set `self.WinScreenRef` _returnvalue))
  (`UserWidget.AddToViewport` _output_get 0)
  (`/Game/LittleBeans/Common/Blueprints/BPFL_PlayerInput.SwitchInputMode` "NewEnumerator1" (`self.WinScreenRef`))
  (`GameplayStatics.SetGamePaused` true)
  (set `self.bIsGamePaused` true))

(event `/Game/LittleBeans/Core/BPI_GameMode.SetCheckpoint`
  (params (CheckpointTransform :type "Transform Structure"))
  ;[1 1 1] Set new checkpoint
  (set `self.CurrentCheckpoint` CheckpointTransform)
  (`KismetSystemLibrary.PrintText` "Checkpoint Set"))

(event `/Game/LittleBeans/Core/BPI_GameMode.SetIsUsingGamepad`
  (params (bIsUsingGamepad :type Boolean))
  ;[1 1 1] Set Gamepad Mode
  (set `self.Is Using Gamepad` bIsUsingGamepad))

(event `/Game/LittleBeans/Gameplay/Pickups/BPI_Pickup.Collected`
  (params (PickupType :type "/Game/LittleBeans/Gameplay/Pickups/Enum_PickupType Enum" :default "NewEnumerator0"))
  ;[1 1 1] Pickup
  (switch `/Game/LittleBeans/Gameplay/Pickups/Enum_PickupType` PickupType
    (:`NewEnumerator0`
      _)
    (:`NewEnumerator1`
      _))
  (`/Engine/EditorBlueprintResources/StandardMacros.IncrementInt` (`self.CurrentPickupCount`)
    (:`  `
      (message `/Game/LittleBeans/Gameplay/Pickups/BPI_Pickup.Collected` (`self.IngameUIRef`) "NewEnumerator0"))))

(event `/Game/LittleBeans/Core/BPI_GameMode.RespawnPlayer`
  (bind _currentcheckpoint_location (`KismetMathLibrary.BreakTransform` (`self.CurrentCheckpoint`)))
  (bind _currentcheckpoint_location_2 (`KismetMathLibrary.BreakTransform` (`self.CurrentCheckpoint`)))
  (bind (_currentcheckpoint_location_3 _currentcheckpoint_rotation) (`KismetMathLibrary.BreakTransform` (`self.CurrentCheckpoint`)))
  ;[1 1 1] Respawn
  (if (!= _currentcheckpoint_location (0.0 0.0 0.0))
    (`self.K2_SetActorLocation` (`GameplayStatics.GetPlayerCharacter` 0) _currentcheckpoint_location_2 false false)
    (`Controller.SetControlRotation` (`GameplayStatics.GetPlayerController` 0) _currentcheckpoint_rotation)))

(event `/Game/LittleBeans/Core/BPI_GameMode.ShowSettings`
  (params (bShow :type Boolean))
  (bind _settingsmenuref (`self.SettingsMenuRef`))
  ;[1 1 1] SettingsMenu
  (if bShow
    (`/Engine/EditorBlueprintResources/StandardMacros.IsValid` _settingsmenuref
      (:`Is Not Valid`
        (bind _returnvalue (`|CreateWidget` "/Game/LittleBeans/UI/WBP_SettingsMenu.WBP_SettingsMenu_C"))
        (bind _output_get (set `self.SettingsMenuRef` _returnvalue))
        (`UserWidget.AddToViewport` _output_get 0)))
    (else
      (`Widget.RemoveFromParent` _settingsmenuref)
      (set `self.SettingsMenuRef` null))))

(event `/Game/LittleBeans/Core/BPI_GameMode.TriggerCheatUI`
  ;[1 1 1] Trigger Cheat UI
  (if (not (`self.bCheatUI`)) :!label _label_2
    (`/Engine/EditorBlueprintResources/StandardMacros.IsValid` (`self.CheatUIRef`)
      (:`Is Valid`
        _)
      (:`Is Not Valid`
        (bind _returnvalue (`|CreateWidget` "/Game/LittleBeans/UI/WBP_CheatUI.WBP_CheatUI_C"))
        (set `self.CheatUIRef` _returnvalue)))
    (`UserWidget.AddToViewport` (`self.CheatUIRef`) 0)
    (`WidgetBlueprintLibrary.SetInputMode_GameAndUIEx` (`GameplayStatics.GetPlayerController` 0) (`self.CheatUIRef`))
    (set `PlayerController.bShowMouseCursor` true (`GameplayStatics.GetPlayerController` 0))
    (set `self.bCheatUI` true)
    (else
      (`Widget.RemoveFromParent` (`self.CheatUIRef`))
      (`WidgetBlueprintLibrary.SetInputMode_GameOnly` (`GameplayStatics.GetPlayerController` 0))
      (set `PlayerController.bShowMouseCursor` false (`GameplayStatics.GetPlayerController` 0))
      (set `self.bCheatUI` false))))

(event `/Game/LittleBeans/Core/BPI_GameMode.SetVolume`
  (params (VolumeType :type "/Game/LittleBeans/Core/Enum_VolumeTypes Enum" :default "NewEnumerator0") (NewVolume :type "Float (double-precision)"))
  ;[1 1 1] Sound Settings
  (switch `/Game/LittleBeans/Core/Enum_VolumeTypes` VolumeType
    (:`NewEnumerator0`
      (bind _output_get (set `self.Master` NewVolume))
      (`FMODBlueprintStatics.VCASetVolume` "/Game/FMOD/VCAs/Master.Master" _output_get))
    (:`NewEnumerator1`
      (bind _output_get_2 (set `self.Music` NewVolume))
      (`FMODBlueprintStatics.VCASetVolume` "/Game/FMOD/VCAs/Music.Music" _output_get_2))
    (:`NewEnumerator2`
      (bind _output_get_3 (set `self.SFX` NewVolume))
      (`FMODBlueprintStatics.VCASetVolume` "/Game/FMOD/VCAs/SFX.SFX" _output_get_3))))

(event `InputAction|CheatMenu`
  (params (Key :type "Key Structure"))
  ;[1 1 1] Trigger Cheat UI
  (:`Pressed`
    (goto _label_2)))

(event `/Game/LittleBeans/Core/BPI_GameMode.TriggerDialgue`
  (params (Speaker :type String) (Text :type String))
  ;[1 1 1] Dialogue
  (`/Engine/EditorBlueprintResources/StandardMacros.IsValid` (`self.DialogueMenuRef`)
    (:`Is Valid`
      _)
    (:`Is Not Valid`
      (message `/Game/LittleBeans/Blueprints/BPI_PlayerCharacter.IsInDialogue` (`GameplayStatics.GetPlayerCharacter` 0) true)
      (bind _returnvalue (`|CreateWidget` "/Game/LittleBeans/UI/WBP_DialgueMenu.WBP_DialgueMenu_C"))
      (bind _output_get (set `self.DialogueMenuRef` _returnvalue))
      (`UserWidget.AddToViewport` _output_get 0)))
  (message `/Game/LittleBeans/UI/BPI_DialogueMenu.ContinueDialogue` (`self.DialogueMenuRef`) Speaker Text))

(event `/Game/LittleBeans/Core/BPI_GameMode.EndDialogue`
  ;[1 1 1] Dialogue
  (`/Engine/EditorBlueprintResources/StandardMacros.IsValid` (`self.DialogueMenuRef`)
    (:`Is Valid`
      (`Widget.RemoveFromParent` (`self.DialogueMenuRef`))
      (set `self.DialogueMenuRef` null)
      (message `/Game/LittleBeans/Blueprints/BPI_PlayerCharacter.is in Activatable Range` (`GameplayStatics.GetPlayerCharacter` 0) null false)
      (message `/Game/LittleBeans/Blueprints/BPI_PlayerCharacter.IsInDialogue` (`GameplayStatics.GetPlayerCharacter` 0) false))))

(fn `GetCurrentPickups`
  (returns (CurrentPickups :type Integer))
  (return (`self.CurrentPickupCount`)))

(fn `GetIsUsingGamepad`
  (returns (bIsUsingGamepad :type Boolean))
  (return (`self.Is Using Gamepad`)))

(fn `GetVolume`
  (params (VolumeType :type "/Game/LittleBeans/Core/Enum_VolumeTypes Enum" :default "NewEnumerator0"))
  (returns (NewVolume :type "Float (double-precision)"))
  (switch `/Game/LittleBeans/Core/Enum_VolumeTypes` VolumeType
    (:`NewEnumerator0`
      (return (`self.Master`)))
    (:`NewEnumerator1`
      (return (`self.Music`)))
    (:`NewEnumerator2`
      (return (`self.SFX`)))))

(fn `UserConstructionScript`)